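; BP_WaterSource is a one-time water source that the player reaches by overlapping it.
; On overlap it casts the actor to ThirdPersonCharacter and, if not yet visited, informs the character that it reached this source.
; It then sets its visited flag, swaps the cube to a visited material, hides the root with its children and spawns a SunPickup effect at its location.
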(event EventBeginPlay)

(event Collision|EventActorBeginOverlap
  (params (OtherActor :type Actor%20Object%20Reference))
  (CallFunction|CheckPlayerJustOverlapped OtherActor))

(event EventTick
  (params (DeltaSeconds :type Float%20%28single-precision%29)))

(fn ConstructionScript)

(fn CheckPlayerJustOverlapped
  (params (Player%20Character%20Actor :type Actor%20Object%20Reference))
  (bind _asthird_person_character (Utilities|Casting|CastToThirdPersonCharacter Player%20Character%20Actor))
  (if (not (Variables|Default|GetAlreadyVisitedOnce)) ; Proceed only if not visited before!
    (Default|InformPlayerReachedtoWaterSource _asthird_person_character self)
    (CallFunction|MarkWaterSourceVisited)))

(fn MarkWaterSourceVisited
  (Utilities|FlowControl|Sequence
    (:then_0
      (Variables|Default|SetAlreadyVisitedOnce true))
    (:then_1
      (Rendering|Material|SetMaterial (Variables|Default|GetCube) 0 "/Game/Materials/MAT_WaterSourceVisited.MAT_WaterSourceVisited"))
    (:then_2
      (Rendering|SetVisibility (Variables|Default|GetDefaultSceneRoot) false true))
    (:then_3
      (Niagara|SpawnSystematLocation "/Game/Effects/SunPickup.SunPickup" (Transformation|GetWorldLocation (Variables|Default|GetDefaultSceneRoot))))))