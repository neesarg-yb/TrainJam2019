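; BP_Collectible is a pickup that grants the third-person character either a double jump or a dash ability, chosen by its CollectibleType.
; The construction script sets the sphere's material to match that type.
; On overlap with the character, it activates the matching ability and has the player controller show the ability UI widget.
; It then hides itself, spawns a Niagara pickup effect and destroys itself.
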(event EventBeginPlay)

(event Collision|EventActorBeginOverlap
  (params (OtherActor :type Actor%20Object%20Reference))
  (CallFunction|TryActivateAbilityforPlayerCharacter OtherActor))

(event EventTick
  (params (DeltaSeconds :type Float%20%28single-precision%29)))

(fn ConstructionScript
  (switch Utilities|FlowControl|Switch|SwitchonENUM_CollectibleType (Variables|Default|GetCollectible%20Type)
    (:NewEnumerator1
      (Rendering|Material|SetMaterial (Variables|Default|GetSphere) 0 "/Game/Materials/MAT_DoubleJumpCollectible.MAT_DoubleJumpCollectible"))
    (:NewEnumerator0
      (Rendering|Material|SetMaterial (Variables|Default|GetSphere) 0 "/Game/Materials/MAT_DashCollectible.MAT_DashCollectible"))))

(fn TryActivateAbilityforPlayerCharacter
  (params (Overlapped%20Actor :type Actor%20Object%20Reference))
  (bind _defaultsceneroot (Variables|Default|GetDefaultSceneRoot))
  (bind _asthird_person_character (Utilities|Casting|CastToThirdPersonCharacter Overlapped%20Actor))
  (Utilities|FlowControl|Sequence
    (:then_0
      (LocalVariables|SetPlayerCharacter _asthird_person_character))
    (:then_1
      (switch Utilities|FlowControl|Switch|SwitchonENUM_CollectibleType (Variables|Default|GetCollectible%20Type)
        (:NewEnumerator1
          (Default|ActivateDoubleJump (LocalVariables|GetPlayerCharacter)))
        (:NewEnumerator0
          (Default|ActivateDash (LocalVariables|GetPlayerCharacter)))))
    (:then_2
      (bind _asbp_player_controller (Utilities|Casting|CastToBP_PlayerController (Game|GetPlayerController 0)))
      (Default|ShowAbilityUIWidget _asbp_player_controller (Variables|Default|GetCollectible%20Type)))
    (:then_3
      (Rendering|SetVisibility _defaultsceneroot false true))
    (:then_4
      (Niagara|SpawnSystematLocation "/Game/Effects/PowerupPickup.PowerupPickup" (Transformation|GetWorldLocation _defaultsceneroot))
      (Actor|DestroyActor self))))