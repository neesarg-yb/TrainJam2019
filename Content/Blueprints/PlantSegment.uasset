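; Actor for one plant segment: a procedurally randomized, curving stem from its own location to a given end point that can be visually grown.
; Setup spaces points by preferred spacing, adding random offsets that taper to zero at both ends and random tangents after the first; EndDirection is stored but unused here.
; Chained spline meshes join the points, each with a dynamic material.
; SetGrowthProgress fills their FillAmount parameters sequentially from start to end.
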(event EventBeginPlay)

(event Collision|EventActorBeginOverlap
  (params (OtherActor :type Actor%20Object%20Reference)))

(event EventTick
  (params (DeltaSeconds :type Float%20%28single-precision%29)))

(fn ConstructionScript)

(fn Setup
  (params (StartDirection :type Vector) (EndPoint :type Vector) (EndDirection :type Vector))
  (bind _output_get (Variables|Default|SetEndPoint EndPoint))
  (Variables|Default|SetEndDirection EndDirection)
  (bind _output_get_2 (LocalVariables|SetSegmentCount (Math|Float|Round (/ (Math|Vector|VectorLength (- _output_get (Transformation|GetWorldLocation (Variables|Default|GetDefaultSceneRoot)))) (Variables|Parameters|GetPreferredSegmentSpacing)))))
  (CallFunction|MakeSegmentPoints _output_get_2 (- _output_get (Transformation|GetWorldLocation (Variables|Default|GetDefaultSceneRoot))) StartDirection)
  (CallFunction|MakeSegmentMeshes))

(fn MakeSegmentMeshes
  (bind _intermediatepoints (Variables|Default|GetIntermediatePoints))
  (bind _intermediatedirections (Variables|Default|GetIntermediateDirections))
  (for _index (range 1 (- (Utilities|Array|Length (Variables|Default|GetIntermediatePoints)) 1))
    (bind _returnvalue (AddComponent|AddSplineMeshComponent true))
    (Transformation|SetMobility _returnvalue "Movable")
    (Transformation|AttachComponentToComponent _returnvalue (Variables|Default|GetDefaultSceneRoot) "None" "SnapToTarget" "SnapToTarget" "SnapToTarget" true)
    (Utilities|Array|Add (Variables|Default|GetSegments) _returnvalue)
    (SplineMesh|SetForwardAxis _returnvalue "Z" false)
    (Components|StaticMesh|SetStaticMesh _returnvalue "/Game/Meshes/PlantSubsegmentMesh.PlantSubsegmentMesh")
    (SplineMesh|SetStartandEnd _returnvalue (Utilities|Array|Get(acopy) _intermediatepoints (- _index 1)) (Utilities|Array|Get(acopy) _intermediatedirections (- _index 1)) (Utilities|Array|Get(acopy) _intermediatepoints _index) (Utilities|Array|Get(acopy) _intermediatedirections _index) true :!class /Script/Engine.SplineMeshComponent)
    (bind _returnvalue_2 (Rendering|Material|CreateDynamicMaterialInstance "/Game/Materials/MAT_Plant.MAT_Plant" "None" :!class /Script/Engine.KismetMaterialLibrary))
    (Utilities|Array|Add (Variables|Default|GetGrowthMaterials) _returnvalue_2)
    (Rendering|Material|SetMaterial _returnvalue 0 _returnvalue_2))
  (return))

(fn MakeSegmentPoints
  (params (SegmentCount :type Integer) (TotalSpan :type Vector) (StartDirection :type Vector))
  (bind _returnvalue (- SegmentCount 1))
  (bind _intermediatedirections (Variables|Default|GetIntermediateDirections))
  (bind _returnvalue_2 (/ TotalSpan _returnvalue))
  (for _index (range 1 SegmentCount)
    (Utilities|Array|Add (Variables|Default|GetIntermediatePoints) (+ (* _returnvalue_2 (- _index 1)) (* (Math|Random|RandomUnitVector) (* (Variables|Parameters|GetPreferredSegmentSpacing) 0.3 (Math|Trig|Sin(Radians) (Math|Float|MultiplybyPi (/ (Math|Conversions|ToFloat(Integer) (- _index 1)) (Math|Conversions|ToFloat(Integer) _returnvalue))))))))
    (if (== _index 1) ; is this the first segment?
      (Utilities|Array|Add _intermediatedirections (* StartDirection (* (Variables|Parameters|GetPreferredSegmentSpacing) (- 1.5 (* (Math|Trig|Sin(Radians) (Math|Float|MultiplybyPi (/ (Math|Conversions|ToFloat(Integer) (- _index 1)) (Math|Conversions|ToFloat(Integer) _returnvalue)))) 0.5))))) ; if it’s the first segment, use the overall starting direction
      (else
        (Utilities|Array|Add _intermediatedirections (* (Math|Random|RandomUnitVectorinConeinDegrees _returnvalue_2 1.1e+02) (* (Variables|Parameters|GetPreferredSegmentSpacing) (- 1.5 (* (Math|Trig|Sin(Radians) (Math|Float|MultiplybyPi (/ (Math|Conversions|ToFloat(Integer) (- _index 1)) (Math|Conversions|ToFloat(Integer) _returnvalue)))) 0.5))))) ; if it’s not the first segment, use a random direction
      )))
  (return))

(fn SetGrowthProgress
  (params (Progress :type Float%20%28single-precision%29))
  (bind _growthmaterials (Variables|Default|GetGrowthMaterials))
  (bind _returnvalue (Utilities|Array|Length _growthmaterials))
  (for _index (range 0 (- _returnvalue 1))
    (Rendering|Material|SetScalarParameterValue (Utilities|Array|Get(acopy) (Variables|Default|GetGrowthMaterials) _index) "FillAmount" (Math|Float|Clamp(Float) (- (* _returnvalue Progress) (Math|Conversions|ToFloat(Integer) _index))) :!class /Script/Engine.MaterialInstanceDynamic)))