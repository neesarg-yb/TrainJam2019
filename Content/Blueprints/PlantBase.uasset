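; PlantBase is a plant actor that grows visibly over time along supplied points, built as a chain of PlantSegment actors.
; Grow spawns a segment per point pair, orienting every one by the first two directions, and rescales progress to the longer approximate length.
; Tick advances progress with an ease-out capped by length, then ApplyGrowthProgress maps it evenly across segments so they grow in sequence.
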(event EventTick
  (params (DeltaSeconds :type Float%20%28single-precision%29))
  (bind _approximatetotallength (Variables|Default|GetApproximateTotalLength))
  (if (and (< (Variables|Default|GetGrowthProgress) 0.99999) (> _approximatetotallength 0.0))
    (Variables|Default|SetGrowthProgress (+ (Variables|Default|GetGrowthProgress) (* DeltaSeconds (Math|Float|Min(Float) (* (- 1.0 (Variables|Default|GetGrowthProgress)) 0.95) (/ 1.2e+03 _approximatetotallength)))))
    (CallFunction|ApplyGrowthProgress)))

(fn ConstructionScript)

(fn Grow
  (params (Positions :type Array%20of%20Vectors) (Directions :type Array%20of%20Vectors))
  (LocalVariables|SetPreviousTotalLength (Variables|Default|GetApproximateTotalLength))
  (for _index (range 0 (- (Utilities|Array|Length Positions) 2))
    (bind _returnvalue (Game|SpawnActorfromClass "/Game/Blueprints/PlantSegment.PlantSegment_C" (Math|Transform|MakeTransform (Utilities|Array|Get(acopy) Positions _index) "0, 0, 0" "1,1,1") "AlwaysSpawn" 0 0))
    (Default|Setup _returnvalue (Utilities|Array|Get(acopy) Directions) (Utilities|Array|Get(acopy) Positions (+ _index 1)) (Utilities|Array|Get(acopy) Directions (+ 0 1)))
    (Utilities|Array|Add (Variables|Default|GetSegments) _returnvalue)
    (Variables|Default|SetApproximateTotalLength (+ (Variables|Default|GetApproximateTotalLength) (Math|Vector|VectorLength (- (Utilities|Array|Get(acopy) Positions _index) (Utilities|Array|Get(acopy) Positions (+ _index 1)))))))
  (Variables|Default|SetGrowthProgress (* (/ (LocalVariables|GetPreviousTotalLength) (Variables|Default|GetApproximateTotalLength)) (Variables|Default|GetGrowthProgress))))

(fn ApplyGrowthProgress
  (bind _segments (Variables|Default|GetSegments))
  (bind _returnvalue (Utilities|Array|Length _segments))
  (for _index (range 0 (- _returnvalue 1))
    (Default|SetGrowthProgress (Utilities|Array|Get(acopy) (Variables|Default|GetSegments) _index) (Math|Float|Clamp(Float) (- (* _returnvalue (Variables|Default|GetGrowthProgress)) (Math|Conversions|ToFloat(Integer) _index))))))